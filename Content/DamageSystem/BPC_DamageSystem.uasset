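; Damage system component that tracks an owner's health and handles healing and incoming damage.
; Heal and TakeDamage adjust Health clamped between zero and MaxHealth, with blocking negating damage entirely.
; Damage that empties Health sets IsDead and calls OnDeath; otherwise an interruptible owner calls OnDamageResponse with the response from DamageInfo.
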(fn Heal
  (params (Amount :type Float%20%28double-precision%29))
  (bind _output_get (Variables|Default|SetHealth (Math|Float|Clamp(Float) (+ (Variables|Default|GetHealth) Amount) 0.0 (Variables|Default|GetMaxHealth))))
  (return _output_get))

(fn TakeDamage
  (params (DamageInfo :type S%20Damage%20Info%20Structure))
  (bind (_amount _damagetype _damageresponse) (Utilities|Struct|BreakS_DamageInfo DamageInfo))
  (if (not (Variables|Default|GetIsBlocking))
    (bind _output_get (Variables|Default|SetHealth (Math|Float|Clamp(Float) (- (Variables|Default|GetHealth) _amount) 0.0 (Variables|Default|GetMaxHealth))))
    (bind _output_get_2 (Variables|Default|SetIsDead (<= _output_get 0.0)))
    (if _output_get_2
      (Default|CallOnDeath)
      (return true)
      (elif (Variables|Default|GetIsInterruptible)
        (Default|CallOnDamageResponse _damageresponse)))))
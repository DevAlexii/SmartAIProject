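; Melee enemy Blueprint that attacks, equips and unequips a sword, and reports its ideal attack and defend ranges.
; Attack plays an uninterruptible montage whose notify runs a forward sphere trace, damaging each hit pawn once.
; Equip and unequip montages use notifies to spawn the sword on a hand socket or destroy it.
; Dispatchers signal when attacks end and weapon changes complete.
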(event EventEquipWeapon
  (bind _notifyname (Animation|Montage|PlayMontage (Variables|Character|GetMesh) "/Game/Characters/Mannequins/Animations/Sword/UnsheatSword_Montage.UnsheatSword_Montage")
    (:OnCompleted
      (Default|CallOnWeaponEquipped))
    (:OnNotifyBegin
      (switch name _notifyname
        (:HoldSword
          (bind _returnvalue (Game|SpawnActorfromClass "/Game/Weapons/BP_Weapon_Sword.BP_Weapon_Sword_C" (Math|Transform|MakeTransform "0, 0, 0") "Undefined" "MultiplyWithRoot" 0 0))
          (Transformation|AttachComponentToComponent _returnvalue (Variables|Character|GetMesh) "hand_r_sword_Socket" "SnapToTarget" "SnapToTarget" "SnapToTarget" true)
          (Variables|Default|SetWeaponActor _returnvalue)
          (Variables|Default|SetIsWieldingWeapon true))))))

(event EventUnequipWeapon
  (bind _notifyname (Animation|Montage|PlayMontage (Variables|Character|GetMesh) "/Game/Characters/Mannequins/Animations/Sword/SheatSword_Montage.SheatSword_Montage")
    (:OnCompleted
      (Default|CallOnWeaponUnquipped))
    (:OnNotifyBegin
      (switch name _notifyname
        (:DropSword
          (Actor|DestroyActor (Variables|Default|GetWeaponActor))
          (Variables|Default|SetIsWieldingWeapon false))))))

(event EventBeginPlay
  (|CallParentFunction))

(event EventAttack
  (bind _returnvalue (Transformation|GetActorLocation))
  (bind _notifyname (Animation|Montage|PlayMontage (Variables|Character|GetMesh) "/Game/Characters/Mannequins/Animations/Sword/AttackBase_Montage.AttackBase_Montage")
    (:then
      (Variables|/Game/DamageSystem/BPC_DamageSystem.BPC_DamageSystem_C|SetIsInterruptible (Variables|Default|GetBPC_DamageSystem) false))
    (:OnCompleted
      (Default|CallOnAttackEnd :!label _label)
      (Variables|/Game/DamageSystem/BPC_DamageSystem.BPC_DamageSystem_C|SetIsInterruptible (Variables|Default|GetBPC_DamageSystem) true))
    (:OnInterrupted
      (goto _label))
    (:OnNotifyBegin
      (switch name _notifyname
        (:Slash
          (bind (_outhits _returnvalue_2) (Collision|MultiSphereTraceForObjects _returnvalue (+ _returnvalue (* (Transformation|GetActorForwardVector) 2e+02)) 2e+01 (Utilities|Array|MakeArray "ObjectTypeQuery3") false 0 "None"))
          (if _returnvalue_2
            (for (_array_element _array_index) _outhits
              (if (> _array_index 0)
                (if (not (Utilities|Array|ContainsItem (Variables|Default|GetHittedActors) (.HitActor (Collision|BreakHitResult _array_element))))
                  (Class|BPIDamagable|TakeDamage(Message) (.HitActor (Collision|BreakHitResult _array_element)) (Utilities|Struct|MakeS_DamageInfo 25.0 "NewEnumerator1") :!label _label_2)
                  (Utilities|Array|AddUnique (Variables|Default|GetHittedActors) (.HitActor (Collision|BreakHitResult _array_element))))
                (else
                  (goto _label_2))))
            (Utilities|Array|Clear (Variables|Default|GetHittedActors))))))))

(fn ConstructionScript
  (|CallParentFunction))

(fn GetIdealRange
  (return 1.5e+02 3.5e+02))
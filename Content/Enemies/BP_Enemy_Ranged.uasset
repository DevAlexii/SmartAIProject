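; BP_Enemy_Ranged is a rifle-wielding enemy that spawns its weapon and attaches it to the hand socket on BeginPlay.
; Attack plays a firing montage whose notify spawns muzzle effects and sound, then damages the AI controller's attack target if a visibility trace finds no blocking hit.
; It calls attack-end when the montage completes or is interrupted, and supplies movement speeds and ideal combat ranges; unequipping is empty.
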(event EventBeginPlay
  (|CallParentFunction)
  (CallFunction|EquipWeapon))

(event EventEquipWeapon
  (bind _returnvalue (Game|SpawnActorfromClass "/Game/Weapons/BP_Weapon_Rifle.BP_Weapon_Rifle_C" (Math|Transform|MakeTransform "0, 0, 0") "Undefined" "MultiplyWithRoot" 0 0))
  (bind _output_get (Variables|Default|SetWeaponActor _returnvalue))
  (Transformation|AttachComponentToComponent _output_get (Variables|Character|GetMesh) "hand_r_Rifle_Socket" "SnapToTarget" "SnapToTarget" "SnapToTarget" true)
  (Variables|Default|SetIsWieldingWeapon true)
  (Default|CallOnWeaponEquipped))

(event EventUnequipWeapon)

(event EventAttack
  (bind _weaponactor (Variables|Default|GetWeaponActor))
  (bind _asbp_weapon_rifle (Utilities|Casting|CastToBP_Weapon_Rifle _weaponactor))
  (bind _muzzlepos (Variables|/Game/Weapons/BP_Weapon_Rifle.BP_Weapon_Rifle_C|GetMuzzlePos _asbp_weapon_rifle))
  (bind _returnvalue (Transformation|GetWorldLocation _muzzlepos))
  (bind _notifyname (Animation|Montage|PlayMontage (Variables|Character|GetMesh) "/Game/Characters/Mannequins/Animations/Rifle/FiringRifle_UE_Montage.FiringRifle_UE_Montage")
    (:OnCompleted
      (Default|CallOnAttackEnd :!label _label))
    (:OnInterrupted
      (goto _label))
    (:OnNotifyBegin
      (switch name _notifyname
        (:Fire
          (Effects|SpawnEmitteratLocation "/Game/StarterContent/Particles/P_Explosion.P_Explosion" _returnvalue "0, 0, 0" "0.200000,0.200000,0.200000")
          (Audio|PlaySoundatLocation "/Game/Weapons/Sound/Rifle.Rifle" _returnvalue "0, 0, 0" 1.0 (Math|Random|RandomFloatinRange 0.8 1.1) 0.0 0 0 0 0)
          (bind _asaic_enemy_base (Utilities|Casting|CastToAIC_Enemy_Base (AI|GetAIController self)))
          (bind _attack_target (Variables|/Game/Enemies/AI/AIC_Enemy_Base.AIC_Enemy_Base_C|GetAttack%20Target _asaic_enemy_base)
            (:then
              (bind _returnvalue_2 (Collision|LineTraceByChannel (Transformation|GetActorLocation (Variables|Default|GetWeaponActor)) (Transformation|GetActorLocation _attack_target) "TraceTypeQuery1" false 0 "None"))
              (if (not _returnvalue_2)
                (Class|BPIDamagable|TakeDamage(Message) _attack_target (Utilities|Struct|MakeS_DamageInfo 2e+01 "NewEnumerator2"))))
            (:else)))))))

(fn ConstructionScript
  (|CallParentFunction))

(fn SetMovementSpeed
  (params (Speed :type E_MovementSpeed%20Enum :default "NewEnumerator0"))
  (bind _output_get (Variables|/Script/Engine.CharacterMovementComponent|SetMaxWalkSpeed (Variables|Character|GetCharacterMovement) (Utilities|Select :Index Speed :NewEnumerator0 0.0 :NewEnumerator1 2e+02 :NewEnumerator2 3e+02 :NewEnumerator3 5e+02)))
  (return _output_get))

(fn GetIdealRange
  (return 6e+02 6e+02))